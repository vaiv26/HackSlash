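; Gameplay ability that plays a hit reaction on the avatar when triggered by a gameplay event carrying a hit result.
; It applies GE_HitReact to the owner and gets a montage for the impact normal through an interface message to the avatar.
; While the montage plays, a brief root motion constant force with gravity pushes along that normal.
; Montage completion, blend-out or cancellation removes the effect and ends the ability.
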(event `self.K2_ActivateAbilityFromEvent`
  (params (EventData :type "GameplayEventData Structure (by ref)"))
  (bind (_eventtag _instigator _target _optionalobject _optionalobject2 _contexthandle) (break `GameplayEventData` EventData))
  (bind (_returnvalue_bblockinghit _returnvalue_binitialoverlap _returnvalue_time _returnvalue_distance _returnvalue_location _returnvalue_impactpoint _returnvalue_normal _returnvalue_impactnormal) (`GameplayStatics.BreakHitResult` (`AbilitySystemBlueprintLibrary.EffectContextGetHitResult` _contexthandle)))
  (if (`AbilitySystemBlueprintLibrary.EffectContextHasHitResult` _contexthandle)
    (set `self.Return Value Impact Normal` _returnvalue_impactnormal)
    (bind _returnvalue (`self.BP_ApplyGameplayEffectToOwner` "/Game/Blueprints/GameplayEffect/GE_HitReact.GE_HitReact_C"))
    (set `self.ActiveGEHitReact` _returnvalue)
    (bind _returnvalue_2 (message `CombatInterface.GetHitReactMontage` (`self.GetAvatarActorFromActorInfo`) (`self.Return Value Impact Normal`)))
    (`AbilityTask_PlayMontageAndWait.CreatePlayMontageAndWaitProxy` "None" _returnvalue_2
      (:`then`
        (`AbilityTask_ApplyRootMotionConstantForce.ApplyRootMotionConstantForce` "None" (`self.Return Value Impact Normal`) 400.0 0.5 false null "SetVelocity" (0.0 0.0 0.0) 0.0 true))
      (:`OnCompleted`
        (`self.BP_RemoveGameplayEffectFromOwnerWithHandle` (`self.ActiveGEHitReact`) :!label _label)
        (`self.K2_EndAbility`))
      (:`OnBlendOut`
        (goto _label))
      (:`OnCancelled`
        (goto _label)))))