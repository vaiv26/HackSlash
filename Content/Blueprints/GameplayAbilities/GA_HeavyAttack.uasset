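; Gameplay ability for a heavy melee attack that plays a montage and ends when it completes.
; MeleeStart and MeleeEnd gameplay events start and clear a fast looping timer that calls PerformTrace.
; PerformTrace sphere-traces between the avatar's weapon tip and tail sockets, fetched through interface messages, ignoring the avatar.
; The trace only draws persistent debug shapes; its hit result is unused.
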(event `self.K2_ActivateAbility`
  (`AbilityTask_PlayMontageAndWait.CreatePlayMontageAndWaitProxy` "None" "/Game/BlendSpaceAndMontages/QuinSAttack3_Montage.QuinSAttack3_Montage"
    (:`then`
      (`|ExecutionSequence`
        (:`then_0`
          (`AbilityTask_WaitGameplayEvent.WaitGameplayEvent` (struct :`TagName` "Event.Montage.Attack.MeleeStart") null
            (:`EventReceived`
              (bind _returnvalue (`KismetSystemLibrary.K2_SetTimer` null "PerformTrace" 0.01 true))
              (set `self.LoopTimer` _returnvalue))))
        (:`then_1`
          (`AbilityTask_WaitGameplayEvent.WaitGameplayEvent` (struct :`TagName` "Event.Montage.Attack.MeleeEnd") null
            (:`EventReceived`
              (`KismetSystemLibrary.K2_ClearAndInvalidateTimerHandle` (`self.LoopTimer`))
              (`KismetSystemLibrary.PrintString` "Timer Cleared"))))))
    (:`OnCompleted`
      (`self.K2_EndAbility`))))

(fn `PerformTrace`
  (bind _returnvalue (`self.GetAvatarActorFromActorInfo`))
  (bind _returnvalue_2 (message `CombatInterface.GetCombatTipSocketLocation` _returnvalue))
  (bind _returnvalue_3 (message `CombatInterface.GetCombatTailSocketLocation` _returnvalue))
  (`KismetSystemLibrary.SphereTraceSingleByProfile` _returnvalue_2 _returnvalue_3 0.0 "Pawn" false (`|MakeArray` _returnvalue) "Persistent"))