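; Player light melee attack gameplay ability that chains three montages on blend out (first, slowed second, first again), committing and ending when finished or interrupted.
; MeleeStart montage events clear the hit list and start a fast looping timer that sphere-traces between the avatar's combat sockets, recording hit actors.
; MeleeEnd stops the timer, then applies directional damage and a melee impact GameplayCue to recorded targets that pass the live-player check.
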(event `self.K2_ActivateAbility`
  (`AbilityTask_PlayMontageAndWait.CreatePlayMontageAndWaitProxy` "None" "/Game/BlendSpaceAndMontages/QuinS_FirstAttack_Montage.QuinS_FirstAttack_Montage"
    (:`then`
      (`|ExecutionSequence` :!label _label
        (:`then_0`
          (`AbilityTask_WaitGameplayEvent.WaitGameplayEvent` (struct :`TagName` "Event.Montage.Attack.MeleeStart") null
            (:`EventReceived`
              (`KismetArrayLibrary.Array_Clear` (`self.HitActors`))
              (bind _returnvalue (`KismetSystemLibrary.K2_SetTimer` null "PerformTrace" 0.01 true))
              (set `self.TimerHandleFor Function` _returnvalue))))
        (:`then_1`
          (`AbilityTask_WaitGameplayEvent.WaitGameplayEvent` (struct :`TagName` "Event.Montage.Attack.MeleeEnd") null
            (:`EventReceived`
              (`KismetSystemLibrary.K2_ClearAndInvalidateTimerHandle` (`self.TimerHandleFor Function`))
              (for _array_element (`self.HitActors`)
                (bind (_hitactor _hitdirection _hitlocation) (break `HitActorData` _array_element))
                (bind _returnvalue_2 (`SlashAbilitySystemLibrary.GetLivePlayers` _hitactor))
                (if _returnvalue_2
                  (`self.CauseDamage` _hitactor _hitdirection)
                  (`self.K2_ExecuteGameplayCueWithParams` (struct :`TagName` "GameplayCue.MeleeImpact") (`AbilitySystemBlueprintLibrary.MakeGameplayCueParameters` 0.0 0.0 (struct) (struct) (struct) (struct) (struct) _hitlocation (0.0 0.0 0.0) null null _hitactor)))))))))
    (:`OnBlendOut`
      (`AbilityTask_PlayMontageAndWait.CreatePlayMontageAndWaitProxy` "None" "/Game/BlendSpaceAndMontages/QuinS_SecondAttack_Montage.QuinS_SecondAttack_Montage" 0.6
        (:`then`
          (goto _label))
        (:`OnBlendOut`
          (`AbilityTask_PlayMontageAndWait.CreatePlayMontageAndWaitProxy` "None" "/Game/BlendSpaceAndMontages/QuinS_FirstAttack_Montage.QuinS_FirstAttack_Montage"
            (:`then`
              (goto _label))
            (:`OnCompleted`
              _)
            (:`OnInterrupted`
              _)
            (:`OnCancelled`
              _)))
        (:`OnInterrupted`
          _)
        (:`OnCancelled`
          _))
      (`self.K2_CommitAbility` :!label _label_2)
      (`self.K2_EndAbility`))
    (:`OnInterrupted`
      (goto _label_2))
    (:`OnCancelled`
      (goto _label_2))))

(fn `PerformTrace`
  (bind _returnvalue (`self.GetAvatarActorFromActorInfo`))
  (bind _returnvalue_2 (message `CombatInterface.GetCombatTipSocketLocation` _returnvalue))
  (bind _returnvalue_3 (message `CombatInterface.GetCombatTailSocketLocation` _returnvalue))
  (bind _outhit (`KismetSystemLibrary.SphereTraceSingle` _returnvalue_3 _returnvalue_2 8.0 "TraceTypeQuery1" false (`|MakeArray` _returnvalue)))
  (bind (_bblockinghit _binitialoverlap _time _distance _location _impactpoint _normal _impactnormal _physmat _hitactor _hitcomponent _hitbonename _bonename _hititem _elementindex _faceindex _tracestart _traceend) (`GameplayStatics.BreakHitResult` _outhit))
  (if _bblockinghit
    (`SlashAbilitySystemLibrary.AddOrUpdateHitActor` (`self.HitActors`) _hitactor (`KismetMathLibrary.Normal` (- (`Actor.K2_GetActorLocation` _hitactor) _traceend)) _location)))