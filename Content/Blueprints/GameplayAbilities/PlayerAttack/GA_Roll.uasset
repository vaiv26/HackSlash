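; GA_Roll is a player gameplay ability that performs a roll by playing the QuinS roll montage.
; A MeleeStart montage event triggers the RollImpact gameplay cue at the avatar's location.
; The ability commits only when the montage completes, is interrupted or is cancelled, then ends.
; A PerformTrace function, not called in this graph, sphere-traces between combat sockets and records hit actors with direction, with persistent debug drawing.
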(event `self.K2_ActivateAbility`
  (`AbilityTask_PlayMontageAndWait.CreatePlayMontageAndWaitProxy` "None" "/Game/BlendSpaceAndMontages/QuinS_Roll_Montage.QuinS_Roll_Montage"
    (:`then`
      (`AbilityTask_WaitGameplayEvent.WaitGameplayEvent` (struct :`TagName` "Event.Montage.Attack.MeleeStart") null
        (:`EventReceived`
          (`self.K2_ExecuteGameplayCueWithParams` (struct :`TagName` "GameplayCue.RollImpact") (`AbilitySystemBlueprintLibrary.MakeGameplayCueParameters` 0.0 0.0 (struct) (struct) (struct) (struct) (struct) (`Actor.K2_GetActorLocation` (`self.GetAvatarActorFromActorInfo`)))))))
    (:`OnCompleted`
      (`self.K2_CommitAbility` :!label _label)
      (`self.K2_EndAbility`))
    (:`OnInterrupted`
      (goto _label))
    (:`OnCancelled`
      (goto _label))))

(fn `PerformTrace`
  (bind _returnvalue (`self.GetAvatarActorFromActorInfo`))
  (bind _returnvalue_2 (message `CombatInterface.GetCombatTipSocketLocation` _returnvalue))
  (bind _returnvalue_3 (message `CombatInterface.GetCombatTailSocketLocation` _returnvalue))
  (bind _outhit (`KismetSystemLibrary.SphereTraceSingleByProfile` _returnvalue_3 _returnvalue_2 8.0 "Pawn" false (`|MakeArray` _returnvalue) "Persistent"))
  (bind (_bblockinghit _binitialoverlap _time _distance _location _impactpoint _normal _impactnormal _physmat _hitactor _hitcomponent _hitbonename _bonename _hititem _elementindex _faceindex _tracestart _traceend) (`GameplayStatics.BreakHitResult` _outhit))
  (if _bblockinghit
    (`SlashAbilitySystemLibrary.AddOrUpdateHitActor` (`self.HitActors`) _hitactor (`KismetMathLibrary.Normal` (- (`Actor.K2_GetActorLocation` _hitactor) _traceend)))))